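; Tank Blueprint that sets up the tank's turret and barrel references and handles player input for camera aiming and firing.
; On BeginPlay it passes the TankBarrel and TankTurret components to setter functions defined outside this graph.
; Azimuth input yaws a gimbal and elevation input pitches the spring arm, keeping the two camera rotations on separate components.
; The TankFire action calls Fire, whose logic also lives outside this graph.
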(event `self.ReceiveBeginPlay`
  (`self.SetBarrelReference` (`self.TankBarrel`))
  (`self.SetTurretReference` (`self.TankTurret`)))

(event `InputAction|TankFire`
  (params (Key :type "Key Structure" :default "AnyKey"))
  (:`Pressed`
    (`self.Fire`)))

(event `InputAxis|AimAzimuth`
  (params (AxisValue :type "Float (single-precision)"))
  ;[1 1 1] Camera Input Binding
  (`SceneComponent.K2_AddLocalRotation` (`self.Azimuth Gimball`) (`KismetMathLibrary.MakeRotator` 0.0 0.0 AxisValue) false false))

(event `InputAxis|AimElevation`
  (params (AxisValue :type "Float (single-precision)"))
  ;[1 1 1] Camera Input Binding
  (`SceneComponent.K2_AddLocalRotation` (`self.SpringArm`) (`KismetMathLibrary.MakeRotator` 0.0 AxisValue) false false))

(fn `UserConstructionScript`)